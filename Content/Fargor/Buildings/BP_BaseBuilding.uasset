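; BP_BaseBuilding is a tower-defence building with health, an owner tag and a list of minions.
; Damage lowers health and updates the health bar widget via MulticastHealth, or triggers Death at zero.
; Death applies a morale penalty through the game state by owner, kills the minions and destroys the building.
; It also passes its owner tag to the possessing AI controller, prunes minion slots and shares a target with minions.
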(event `self.ReceiveBeginPlay`)

(event `self.ReceiveTick`
  (params (DeltaSeconds :type "Float (single-precision)")))

(event `self.ReceiveAnyDamage`
  (params (Damage :type "Float (single-precision)") (DamageType :type "DamageType Object Reference") (InstigatedBy :type "Controller Object Reference") (DamageCauser :type "Actor Object Reference"))
  (`self.ReceiveDamage` Damage))

(event `self.ReceivePossessed`
  (params (NewController :type "Controller Object Reference"))
  (bind _asbp_tower_aicontroller (cast `/Game/Fargor/Buildings/Towers/TowersAI/BP_TowerAIController` NewController))
  (set `/Game/Fargor/Buildings/Towers/TowersAI/BP_TowerAIController.OwnerTag` (`self.OwnerTag`) _asbp_tower_aicontroller))

(event `MulticastHealth`
  (bind _ashealth_bar (cast `/Game/Fargor/UI/Game/World/HealthBar` (`WidgetComponent.GetWidget` (`self.HealthBar`))))
  (`/Game/Fargor/UI/Game/World/HealthBar.UpdateHealth` _ashealth_bar (`self.Health`) (`self.MaxHealth`)))

(fn `CheckMinionsSlots`
  (returns (NewLength :type Integer))
  (locals (CleanSlots :type "Array of /Game/Fargor/Characters/BP_BaseCharacter Object Reference"))
  (bind _cleanslots (`local.CleanSlots`))
  (for _array_element (`self.Minions`)
    (if (not (== _array_element null))
      (`KismetArrayLibrary.Array_Add` _cleanslots _array_element)))
  (`KismetArrayLibrary.Array_Resize` (`self.Minions`) (`KismetArrayLibrary.Array_Length` _cleanslots))
  (bind _output_get (set `self.Minions` _cleanslots))
  (return (`KismetArrayLibrary.Array_Length` _output_get)))

(fn `Death`
  (bind _asbp_tower_defence_game_state (cast `/Game/Fargor/TowerGameMode/BP_TowerDefenceGameState` (`GameplayStatics.GetGameState`)))
  (`/Game/Fargor/TowerGameMode/BP_TowerDefenceGameState.AddToMoral` _asbp_tower_defence_game_state (* (`self.MoralValue`) -1) (== "Player 0" (`self.OwnerTag`)))
  (for _array_element (`self.Minions`)
    (`/Engine/EditorBlueprintResources/StandardMacros.IsValid` _array_element
      (:`Is Valid`
        (`/Game/Fargor/Characters/BP_BaseCharacter.Death` _array_element))))
  (`self.K2_DestroyActor`))

(fn `FillHealth`
  (set `self.Health` (`self.MaxHealth`)))

(fn `PassTargetToMinions`
  (for _array_element (`self.Minions`)
    (bind _asbp_minion (cast `/Game/Fargor/Characters/Minions/BP_Minion` _array_element))
    (set `/Game/Fargor/Characters/Minions/BP_Minion.TargetForMinion` (`self.TargetForMinions`) _asbp_minion)))

(fn `ReceiveDamage`
  (params (Damage :type "Float (double-precision)"))
  (bind _output_get (set `self.Health` (- (`self.Health`) Damage)))
  (if (<= _output_get 0.0)
    (`self.Death`)
    (else
      (`self.MulticastHealth`))))

(fn `UserConstructionScript`
  (`self.FillHealth`))