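; BP_BaseCharacter is a tower defence character with health, an attack and widgets for health and team.
; Damage either updates the health bar through MulticastHealth or triggers Death, which applies negative morale via the game state by player tag and destroys the actor.
; Shoot passes damage and bullet lifetime to BPBaseAttack before attacking.
; Team indicators take the owner tag directly or after a timer; the runtime widget-creation path is called only from unwired nodes.
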(event `SetTeamColorOnMulticast`
  (params (OwnerTag :type Name))
  (bind _returnvalue (`AddComponent|NODE_AddWidgetComponent-0` :`RelativeTransform` (`KismetMathLibrary.MakeTransform` (0.0 0.0 70.0))))
  (bind _returnvalue_2 (`|CreateWidget` "/Game/Fargor/UI/Game/World/TeamIdicator.TeamIdicator_C" (`GameplayStatics.GetPlayerController` 0) OwnerTag))
  (`WidgetComponent.SetWidget` _returnvalue _returnvalue_2)
  (`WidgetComponent.SetWidgetSpace` _returnvalue "Screen"))

(event `self.ReceivePossessed`
  (params (NewController :type "Controller Object Reference")))

(event `SetTeamColorOnServer`
  (params (OwnerTag :type Name))
  (`self.SetTeamColorOnMulticast` OwnerTag))

(event `self.ReceiveBeginPlay`)

(event `SetTeamColor`
  (bind _asteam_idicator (cast `/Game/Fargor/UI/Game/World/TeamIdicator` (`WidgetComponent.GetWidget` (`self.TeamIndicator`)) :!label _label))
  (set `/Game/Fargor/UI/Game/World/TeamIdicator.OwnerTag` (`self.OwnerTag`) _asteam_idicator))

(event `ActualSetTeamColor`
  (goto _label))

(event `self.ReceiveTick`
  (params (DeltaSeconds :type "Float (single-precision)")))

(event `DelayedTeamColor`
  (params (Time :type "Float (double-precision)"))
  (`KismetSystemLibrary.K2_SetTimerDelegate` (delegate `ActualSetTeamColor`) Time))

(event `self.ReceiveAnyDamage`
  (params (Damage :type "Float (single-precision)") (DamageType :type "DamageType Object Reference") (InstigatedBy :type "Controller Object Reference") (DamageCauser :type "Actor Object Reference"))
  (bind _output_get (set `self.Health` (- (`self.Health`) Damage)))
  (if (<= _output_get 0.0)
    (`self.Death`)
    (else
      (`self.MulticastHealth`))))

(event `MulticastHealth`
  (bind _ashealth_bar (cast `/Game/Fargor/UI/Game/World/HealthBar` (`WidgetComponent.GetWidget` (`self.HealthBar`))))
  (`/Game/Fargor/UI/Game/World/HealthBar.UpdateHealth` _ashealth_bar (`self.Health`) (`self.MaxHealth`)))

(fn `Death`
  (bind _asbp_tower_defence_game_state (cast `/Game/Fargor/TowerGameMode/BP_TowerDefenceGameState` (`GameplayStatics.GetGameState`)))
  (`/Game/Fargor/TowerGameMode/BP_TowerDefenceGameState.AddToMoral` _asbp_tower_defence_game_state (* (`self.Moral Value`) -1) (== "Player 0" (`|GetArrayItem` (`self.Tags`))))
  (`self.K2_DestroyActor`))

(fn `FillHealth`
  (set `self.Health` (`self.MaxHealth`)))

(fn `Shoot`
  (bind _bp_baseattack (`self.BP_BaseAttack`))
  (set `/Game/Fargor/Components/Attacks/BP_BaseAttack.Damage` (`self.BaseDamage`) _bp_baseattack)
  (set `/Game/Fargor/Components/Attacks/BP_BaseAttack.BulletLifetime` (`self.BulletLifetime`) _bp_baseattack)
  (`/Game/Fargor/Components/Attacks/BP_BaseAttack.Attack` _bp_baseattack))

(fn `TagAttack`
  (params (OwnersName :type Name))
  (set `/Game/Fargor/Components/Attacks/BP_BaseAttack.OwnersTag` OwnersName (`self.BP_BaseAttack`)))

(fn `UserConstructionScript`
  (`self.FillHealth`))