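; BP_Bullet is a projectile actor that damages what it hits and expires after a lifetime counted down on Tick.
; Sphere hits destroy it, sparing actors that share its first tag.
; That tag's last digit selects the instigating player controller.
; Damage adds BaseDamage to a morale bonus from the tower defence game state, which counts Moral0 or Moral1 only when that value equals the digit, scaled by DivideMoral.
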(event `self.ReceiveBeginPlay`)

(event `self.ReceiveTick`
  (params (DeltaSeconds :type "Float (single-precision)"))
  (bind _output_get (set `self.MaxLifetime` (- (`self.MaxLifetime`) DeltaSeconds)))
  (if (<= _output_get 0.0)
    (`self.K2_DestroyActor`)))

(event `self.Sphere.OnComponentHit`
  (params (HitComponent :type "PrimitiveComponent Object Reference") (OtherActor :type "Actor Object Reference") (OtherComp :type "PrimitiveComponent Object Reference") (NormalImpulse :type "Vector Structure") (Hit :type "HitResult Structure (by ref)"))
  (bind _tags (`self.Tags`))
  (bind _returnvalue (`KismetStringLibrary.Conv_StringToInt` (`KismetStringLibrary.Right` (`KismetStringLibrary.Conv_NameToString` (`|GetArrayItem` (`self.Tags`))) 1)))
  ;[1 1 1] Damage Target
  (`/Engine/EditorBlueprintResources/StandardMacros.IsValid` OtherActor
    (:`Is Valid`
      (if (> (`KismetArrayLibrary.Array_Length` _tags) 0)
        (if (`self.ActorHasTag` OtherActor (`|GetArrayItem` _tags))
          (`self.K2_DestroyActor` :!label _label)
          (else
            (bind _asbp_tower_defence_game_state (cast `/Game/Fargor/TowerGameMode/BP_TowerDefenceGameState` (`GameplayStatics.GetGameState`))
              (:`then`
                (bind _moral_0 (`/Game/Fargor/TowerGameMode/BP_TowerDefenceGameState.Moral_0` _asbp_tower_defence_game_state))
                (bind _moral_1 (`/Game/Fargor/TowerGameMode/BP_TowerDefenceGameState.Moral_1` _asbp_tower_defence_game_state))
                (`GameplayStatics.ApplyDamage` OtherActor (+ (`KismetMathLibrary.Conv_IntToDouble` (/ (+ (* _moral_0 (`KismetMathLibrary.Conv_BoolToInt` (== _returnvalue _moral_0))) (* _moral_1 (`KismetMathLibrary.Conv_BoolToInt` (== _returnvalue _moral_1)))) (`self.DivideMoral`))) (`self.BaseDamage`)) (`GameplayStatics.GetPlayerController` _returnvalue) null "/Script/Engine.DamageType")
                (`self.K2_DestroyActor`))
              (:`CastFailed`
                (goto _label)))))
        (else
          (goto _label))))
    (:`Is Not Valid`
      (goto _label))))

(fn `UserConstructionScript`)