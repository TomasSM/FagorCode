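; Game mode for the tower defence mode that assigns each joining player a start point and an owner identity.
; The ChoosePlayerStart override picks the first PlayerStart not tagged "Taken", then marks it taken.
; The start's index modulo two yields a Player0 or Player1 tag, written to the PlayerState's tags and BP_TowerDefencePlayerState's OwnershipTag.
; It then calls NewPlayerHasEnteredTheGame and returns that start.
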(fn `ChoosePlayerStart`
  (params (Player :type "Controller Object Reference"))
  (returns (ReturnValue :type "Actor Object Reference"))
  (bind _playerstate (`Controller.PlayerState` Player))
  (bind _outactors (`GameplayStatics.GetAllActorsOfClass` "/Script/Engine.PlayerStart"))
  (for (_array_element _array_index) _outactors
    (if (not (== (`PlayerStart.PlayerStartTag` _array_element) "Taken"))
      (bind _returnvalue (`KismetStringLibrary.Conv_StringToName` (`KismetStringLibrary.BuildString_Int` "Player " "" (mod _array_index 2))))
      (`KismetArrayLibrary.Array_Add` (`Actor.Tags` _playerstate) _returnvalue)
      (bind _asbp_tower_defence_player_state (cast `/Game/Fargor/TowerGameMode/BP_TowerDefencePlayerState` _playerstate)
        (:`then`
          (set `/Game/Fargor/TowerGameMode/BP_TowerDefencePlayerState.Ownership Tag` _returnvalue _asbp_tower_defence_player_state)
          (break))
        (:`CastFailed`
          (break)))))
  (set `PlayerStart.PlayerStartTag` "Taken" _array_element)
  (`self.NewPlayerHasEnteredTheGame`)
  (return _array_element))

(fn `UserConstructionScript`)