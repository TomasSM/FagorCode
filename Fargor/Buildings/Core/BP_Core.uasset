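; BP_Core is the core building in a tower defence game, whose death finishes the match.
; It overrides ReceiveDamage to fire an UpdateHealthUI event, empty here, before running the parent damage logic.
; Its Death override passes the actor's first tag to FinishGame on BP_TowerDefenceGameState, then calls the parent; a failed cast skips both.
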(event `UpdateHealthUI`)

(event `self.ReceiveBeginPlay`
  (`parent.ReceiveBeginPlay`))

(fn `Death`
  (bind _asbp_tower_defence_game_state (cast `/Game/Fargor/TowerGameMode/BP_TowerDefenceGameState` (`GameplayStatics.GetGameState`)))
  (`/Game/Fargor/TowerGameMode/BP_TowerDefenceGameState.FinishGame` _asbp_tower_defence_game_state (`|GetArrayItem` (`self.Tags`)))
  (`parent.Death`))

(fn `ReceiveDamage`
  (params (Damage :type "Float (double-precision)"))
  (`self.UpdateHealthUI`)
  (`parent.ReceiveDamage` Damage))

(fn `UserConstructionScript`
  (`parent.UserConstructionScript`))