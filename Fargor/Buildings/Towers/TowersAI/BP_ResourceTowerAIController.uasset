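; AI controller for resource towers that reacts to perceived actors tagged Resource.
; It overrides the parent's perception hook, casts the blackboard SelfActor to BP_DefenceTower, sets the resource as TargetForMinions and passes it to the minions.
; The parent's perception handling runs afterwards, and also for untagged actors, but is skipped if that cast fails.
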(fn `SlotForChildrenAIPerception`
  (params (Actor :type "Actor Object Reference") (Stimulus :type "AIStimulus Structure"))
  (if (`self.ActorHasTag` Actor "Resource")
    (bind _asbp_defence_tower (cast `/Game/Fargor/Buildings/Towers/BP_DefenceTower` (`BlackboardComponent.GetValueAsObject` (`self.Blackboard`) (`self.SelfActor`))))
    (set `/Game/Fargor/Buildings/BP_BaseBuilding.TargetForMinions` Actor _asbp_defence_tower)
    (`/Game/Fargor/Buildings/BP_BaseBuilding.PassTargetToMinions` _asbp_defence_tower))
  (`parent.SlotForChildrenAIPerception` Actor Stimulus))

(fn `UserConstructionScript`
  (`parent.UserConstructionScript`))