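; AI controller for tower buildings that copies the building's owner tag on possess and runs the tower behavior tree.
; Perception updates call an empty hook for child classes, then pass an ownership check and skip dead players.
; The distance check measures the current Blackboard target, not the sensed actor.
; The sensed actor becomes Target when none exists or the current one is in range; otherwise Target is cleared.
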(event `self.ReceivePossess`
  (params (PossessedPawn :type "Pawn Object Reference"))
  (bind _asbp_base_building (cast `/Game/Fargor/Buildings/BP_BaseBuilding` PossessedPawn))
  (`KismetArrayLibrary.Array_Add` (`self.Tags`) (`/Game/Fargor/Buildings/BP_BaseBuilding.OwnerTag` _asbp_base_building))
  (`self.RunBehaviorTree` "/Game/Fargor/Buildings/Towers/TowersAI/TowerBehaviorTree.TowerBehaviorTree"))

(event `self.AIPerception.OnTargetPerceptionUpdated`
  (params (Actor :type "Actor Object Reference") (Stimulus :type "AIStimulus Structure"))
  (`self.SlotForChildrenAIPerception` Actor Stimulus)
  (if (`self.CheckOwner` Actor Stimulus Actor)
    (bind _asbp_player (cast `/Game/Fargor/Characters/Player/BP_Player` Actor)
      (:`then`
        (if (not (`/Game/Fargor/Characters/Player/BP_Player.Dead` _asbp_player))
          (bind _returnvalue (`self.CheckDistance` :!label _label)
            (:`then`
              (if _returnvalue
                (`BlackboardComponent.SetValueAsObject` (`self.Blackboard`) (`self.Target`) Actor :!label _label_2)
                (else
                  (`BlackboardComponent.SetValueAsObject` (`self.Blackboard`) (`self.Target`) null))))
            (:`ActorNotFound`
              (goto _label_2)))))
      (:`CastFailed`
        (goto _label)))))

(fn `SlotForChildrenAIPerception`
  (params (Actor :type "Actor Object Reference") (Stimulus :type "AIStimulus Structure")))

(fn `UserConstructionScript`)