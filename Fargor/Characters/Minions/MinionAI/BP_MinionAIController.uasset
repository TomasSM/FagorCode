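; AI controller for BP_Minion that runs the minion behavior tree and picks its targets from AI perception.
; On blackboard setup it stores the minion's home and main target and copies the owner tag to itself.
; Perceived actors passing CheckOwner become Target based on CheckDistance or a MainTarget comparison, excluding dead players; otherwise Target clears.
; Each pick resets CanChooseTarget until a five-second timer restores it.
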(event `self.ReceivePossess`
  (params (PossessedPawn :type "Pawn Object Reference"))
  (bind _asbp_minion (cast `/Game/Fargor/Characters/Minions/BP_Minion` PossessedPawn))
  (set `self.As BP Minion` _asbp_minion)
  (`self.RunBehaviorTree` "/Game/Fargor/Characters/Minions/MinionAI/MinionBehaviorTree.MinionBehaviorTree"))

(event `self.OnUsingBlackBoard`
  (params (BlackboardComp :type "BlackboardComponent Object Reference") (BlackboardAsset :type "BlackboardData Object Reference"))
  (bind _as_bp_minion (`self.As BP Minion`))
  (bind _home (`/Game/Fargor/Characters/Minions/BP_Minion.Home` _as_bp_minion))
  ;[1 1 1] Set AI values
  (`BlackboardComponent.SetValueAsObject` (`self.Blackboard`) (`self.HomeActor`) _home)
  (`BlackboardComponent.SetValueAsVector` (`self.Blackboard`) (`self.Home`) (`self.K2_GetActorLocation` _home))
  (`BlackboardComponent.SetValueAsObject` (`self.Blackboard`) (`self.MainTarget`) (`/Game/Fargor/Characters/Minions/BP_Minion.TargetForMinion` _as_bp_minion))
  (`KismetArrayLibrary.Array_Add` (`self.Tags`) (`/Game/Fargor/Characters/BP_BaseCharacter.OwnerTag` _as_bp_minion)))

(event `self.ReceiveBeginPlay`)

(event `CanChooseANewTarget`
  ;[1 1 1] Checks for a target
  (set `self.CanChooseTarget` true))

(event `self.AIPerception.OnTargetPerceptionUpdated`
  (params (Actor :type "Actor Object Reference") (Stimulus :type "AIStimulus Structure"))
  (bind _returnvalue (or (`self.CheckDistance` Actor) (!= (`BlackboardComponent.GetValueAsObject` (`self.Blackboard`) (`self.MainTarget`)) null)))
  ;[1 1 1] Checks for a target
  (if (`self.CheckOwner` Stimulus Actor)
    (bind _asbp_player (cast `/Game/Fargor/Characters/Player/BP_Player` Actor)
      (:`then`
        (if (and _returnvalue (not (`/Game/Fargor/Characters/Player/BP_Player.Dead` _asbp_player)))
          (`BlackboardComponent.SetValueAsObject` (`self.Blackboard`) (`self.Target`) Actor :!label _label)
          (set `self.CanChooseTarget` false)
          (`KismetSystemLibrary.K2_SetTimerDelegate` (delegate `CanChooseANewTarget`) 5.0)
          (else
            (`BlackboardComponent.SetValueAsObject` (`self.Blackboard`) (`self.Target`) null :!label _label_2)
            (set `self.CanChooseTarget` true))))
      (:`CastFailed`
        (if _returnvalue
          (goto _label)
          (else
            (goto _label_2)))))))

(fn `UserConstructionScript`)