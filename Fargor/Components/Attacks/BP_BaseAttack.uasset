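; BP_BaseAttack is a base attack component that aims itself at a target and fires BP_Bullet projectiles on a reload timer.
; Tick counts down the reload and, while tracking, calls AimOnServer, which smoothly rotates toward a point slightly above the target's location.
; AttackOnServer calls Attack, which spawns a bullet at the component's transform, tags it with OwnersTag and passes damage and lifetime with default fallbacks.
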(event `self.ReceiveTick`
  (params (DeltaSeconds :type "Float (single-precision)"))
  (set `self.ReloadTimer` (- (`self.ReloadTimer`) DeltaSeconds))
  (if (`self.Track`)
    (`self.AimOnServer` (`Actor.K2_GetActorLocation` (`self.TrackTarget`)))))

(event `AttackOnServer`
  (`self.Attack`))

(event `AimOnServer`
  (params (Target :type "Vector Structure (by ref)"))
  (`self.Aim` Target))

(fn `Aim`
  (params (Target :type "Vector Structure (by ref)"))
  (`self.K2_SetWorldRotation` (`KismetMathLibrary.RInterpTo` (`self.K2_GetComponentRotation`) (`KismetMathLibrary.FindLookAtRotation` (`self.K2_GetComponentLocation`) (`KismetMathLibrary.MakeVector` (.x Target) (.y Target) (+ (.z Target) 50.0))) 0.05 4.0)))

(fn `Attack`
  (returns (ReturnValue :type "/Game/Fargor/Components/Attacks/BP_Bullet Object Reference"))
  (if (<= (`self.ReloadTimer`) 0.0)
    (bind _returnvalue (`|SpawnActorFromClass` "/Game/Fargor/Components/Attacks/BP_Bullet.BP_Bullet_C" (`KismetMathLibrary.MakeTransform` (.location (`self.K2_GetComponentToWorld`)) (.rotation (`self.K2_GetComponentToWorld`))) "AlwaysSpawn" "OverrideRootScale" (`Actor.GetOwner` (`self.GetOwner`)) (`self.SelectValue` (`self.Damage`) (`self.DefaultDamage`)) (`self.SelectValue` (`self.BulletLifetime`) (`self.DefaultBulletLifetime`)) null))
    (`KismetArrayLibrary.Array_Add` (`Actor.Tags` _returnvalue) (`self.OwnersTag`))
    (set `self.ReloadTimer` (`self.ReloadSpeed`))
    (set `self.LastBullet` _returnvalue)
    (return _returnvalue)))

(fn `StartTracking`
  (params (TrackTarget :type "Actor Object Reference"))
  (set `self.TrackTarget` TrackTarget)
  (set `self.Track` true))

(fn `StopTracking`
  (set `self.Track` false))