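; Base spawn point component that spawns minions and their AI controllers at its world location and rotation.
; SpawnOnServer calls Spawn and stores the resulting minion.
; Spawn creates the configured class and, if it is a BP_Minion, sets its target, owner tag, home actor and team color.
; It then spawns the configured AI class, passes it the owner tag and has it possess the minion.
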(event `self.ReceiveBeginPlay`)

(event `SpawnOnServer`
  (params (TargetForMinion :type "Actor Object Reference") (OwnersName :type "Name (by ref)"))
  (bind _newspawn (`self.Spawn` TargetForMinion OwnersName))
  (set `self.NewActorOnServer` _newspawn))

(fn `Spawn`
  (params (TargetForMinion :type "Actor Object Reference") (OwnersName :type "Name (by ref)"))
  (returns (NewSpawn :type "Actor Object Reference"))
  (bind _returnvalue (`KismetMathLibrary.MakeTransform` (.location (`self.K2_GetComponentToWorld`)) (.rotation (`self.K2_GetComponentToWorld`))))
  (bind _returnvalue_2 (`|SpawnActorFromClass` (`self.SpawnClass`) _returnvalue "AdjustIfPossibleButAlwaysSpawn" "OverrideRootScale" null null))
  (bind _asbp_minion (cast `/Game/Fargor/Characters/Minions/BP_Minion` _returnvalue_2)
    (:`then`
      (`KismetArrayLibrary.Array_Add` (`Actor.Tags` _returnvalue_2) OwnersName)
      (set `/Game/Fargor/Characters/Minions/BP_Minion.TargetForMinion` TargetForMinion _asbp_minion)
      (`/Game/Fargor/Characters/BP_BaseCharacter.TagAttack` _asbp_minion OwnersName)
      (set `/Game/Fargor/Characters/BP_BaseCharacter.OwnerTag` OwnersName _asbp_minion)
      (set `/Game/Fargor/Characters/Minions/BP_Minion.Home` (`self.GetOwner`) _asbp_minion)
      (`/Game/Fargor/Characters/BP_BaseCharacter.SetTeamColor` _asbp_minion)
      (bind _returnvalue_3 (`|SpawnActorFromClass` (`self.SpawnAiClass`) _returnvalue "AlwaysSpawn" "OverrideRootScale" null null))
      (set `/Game/Fargor/Characters/Minions/MinionAI/BP_MinionAIController.OwnerTag` OwnersName _returnvalue_3)
      (`Controller.Possess` _returnvalue_3 _asbp_minion))
    (:`CastFailed`
      _))
  (return _asbp_minion))