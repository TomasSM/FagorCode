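; Game state for a tower defence mode that builds towers, tracks two morale values and announces game end.
; BuildTower spawns a class picked by building enum, stamps the owner's first tag on it and its attack component, and passes on the minion target.
; AddToMoral clamps the selected morale value between limits.
; FinishGame calls a multicast-named event that notifies each player state of the defeated player.
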(event `FinishGameOnMulticast`
  (params (DefeatedPlayer :type Name))
  (for _array_element (`self.PlayerArray`)
    (bind _asbp_tower_defence_player_state (cast `/Game/Fargor/TowerGameMode/BP_TowerDefencePlayerState` _array_element))
    (`/Game/Fargor/TowerGameMode/BP_TowerDefencePlayerState.GameIsFinished` _asbp_tower_defence_player_state DefeatedPlayer)))

(fn `AddToMoral`
  (params (ValueToAdd :type Integer) (Moral_0 :type Boolean :default true))
  (if Moral_0
    (set `self.Moral_0` (`KismetMathLibrary.Clamp` (+ (`self.Moral_0`) ValueToAdd) (`self.MinMoral`) (`self.MaxMoral`)))
    (else
      (set `self.Moral_1` (`KismetMathLibrary.Clamp` (+ (`self.Moral_1`) ValueToAdd) (`self.MinMoral`) (`self.MaxMoral`))))))

(fn `BuildTower`
  (params (Building :type "/Game/Fargor/Buildings/Buildings Enum" :default "NewEnumerator0") (Position :type "Transform Structure") (Owner :type "Actor Object Reference") (TargetForMinions :type "Actor Object Reference"))
  (bind _output (`|GetArrayItem` (`Actor.Tags` Owner)))
  (bind _returnvalue (`|SpawnActorFromClass` (`|GetArrayItem` (`self.BuildingsToBuild`) (- (`KismetMathLibrary.Conv_ByteToInt` Building) 1)) Position "AdjustIfPossibleButAlwaysSpawn" "OverrideRootScale" Owner _output null))
  (`KismetArrayLibrary.Array_Add` (`Actor.Tags` _returnvalue) _output)
  (bind _output_get (set `/Game/Fargor/Buildings/BP_BaseBuilding.OwnerTag` _output _returnvalue))
  (set `/Game/Fargor/Buildings/BP_BaseBuilding.TargetForMinions` TargetForMinions _returnvalue)
  (`/Game/Fargor/Buildings/BP_BaseBuilding.PassTargetToMinions` _returnvalue)
  (set `/Game/Fargor/Components/Attacks/BP_BaseAttack.OwnersTag` _output_get (`/Game/Fargor/Buildings/BP_BaseBuilding.BP_BaseAttack` _returnvalue)))

(fn `FinishGame`
  (params (DefeatedPlayer :type Name))
  (`self.FinishGameOnMulticast` DefeatedPlayer))

(fn `UserConstructionScript`)