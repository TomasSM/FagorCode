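; Player controller for a multiplayer tower defence game, handling pawn movement, mouse-facing, attacks, tower building and demolition, and the HUD.
; A Normal/Build mode switches the main click between firing and placing towers through the game state, capped by a player-count-based limit.
; On possession it copies the PlayerState's team tag for ownership checks and picks an enemy core as minion target.
; A PlayerState dispatcher triggers the HUD's end-game text.
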(event `self.ReceiveBeginPlay`
  (`self.StartUI`)
  (bind _asbp_tower_defence_game_mode (cast `/Game/Fargor/TowerGameMode/BP_TowerDefenceGameMode` (`GameplayStatics.GetGameMode`)))
  (add `/Game/Fargor/TowerGameMode/BP_TowerDefenceGameMode.NewPlayerHasEnteredTheGame` _asbp_tower_defence_game_mode (delegate `NewPlayer`)))

(event `StartUI`
  ;[1 1 1] Create the game's HUD
  (bind _returnvalue (`|CreateWidget` "/Game/Fargor/UI/Game/HUD/TowerDefenceUI.TowerDefenceUI_C" self))
  (bind _output_get (set `self.Viewport` _returnvalue))
  (`UserWidget.AddToViewport` _output_get 0))

(event `InputVectorAxis|Mouse2D`
  (params (AxisValue :type "Vector Structure"))
  ;[1 1 1] Character Turn to face mouse position
  (`self.CalculatePlayerTurn`))

(event `NewPlayer`
  ;[1 1 1] Deals with new players entering the game
  ;;[1 1 1] Sets how many towers each player have
  (bind _returnvalue (`GameModeBase.GetNumPlayers` (`GameplayStatics.GetGameMode`)))
  (set `self.MaxTowers` (/ 12 (/ _returnvalue 2))))

(event `InputAction|Cancel`
  (params (Key :type "Key Structure"))
  ;[1 1 1] Cancelation
  (:`Pressed`
    (set `self.Mode` "NewEnumerator0")))

(event `InputAxis|Up`
  (params (AxisValue :type "Float (single-precision)"))
  (bind _returnvalue (`self.K2_GetPawn`))
  ;[1 1 1] Movement
  (if (`KismetSystemLibrary.IsValid` _returnvalue)
    (`Pawn.AddMovementInput` _returnvalue (1.0 0.0 0.0) AxisValue false)))

(event `InputAxis|Right`
  (params (AxisValue :type "Float (single-precision)"))
  (bind _returnvalue (`self.K2_GetPawn`))
  ;[1 1 1] Movement
  (if (`KismetSystemLibrary.IsValid` _returnvalue)
    (`Pawn.AddMovementInput` _returnvalue (0.0 1.0 0.0) AxisValue false)))

(event `InputAction|Exit Game`
  (params (Key :type "Key Structure"))
  ;[1 1 1] Quiting the game
  (:`Released`
    (`DestroySessionCallbackProxy.DestroySession` self
      (:`OnSuccess`
        (`KismetSystemLibrary.QuitGame` self "Quit")))))

(event `self.ReceivePossess`
  (params (PossessedPawn :type "Pawn Object Reference"))
  (bind _output (`|GetArrayItem` (`Actor.Tags` (`self.PlayerState`))))
  ;[1 1 1] Adding ownership tags
  (set `self.Possessed Pawn` PossessedPawn)
  (`KismetArrayLibrary.Array_Add` (`self.Tags`) _output)
  (`KismetArrayLibrary.Array_Add` (`Actor.Tags` PossessedPawn) _output)
  (bind _asbp_player (cast `/Game/Fargor/Characters/Player/BP_Player` PossessedPawn))
  (`/Game/Fargor/Characters/BP_BaseCharacter.TagAttack` _asbp_player _output)
  (set `/Game/Fargor/Characters/BP_BaseCharacter.OwnerTag` _output _asbp_player)
  (`/Game/Fargor/Characters/BP_BaseCharacter.DelayedTeamColor` _asbp_player 10.0)
  (bind _outactors (`GameplayStatics.GetAllActorsOfClass` "/Game/Fargor/Buildings/Core/BP_Core.BP_Core_C"))
  (for _array_element _outactors
    (if (!= (`|GetArrayItem` (`Actor.Tags` _array_element)) _output)
      (break)))
  (set `self.TargetForAttack` _array_element)
  ;[1 1 1] Set up end game screen activation
  (bind _asbp_tower_defence_player_state (cast `/Game/Fargor/TowerGameMode/BP_TowerDefencePlayerState` (`self.PlayerState`)))
  (add `/Game/Fargor/TowerGameMode/BP_TowerDefencePlayerState.GameIsFinished` _asbp_tower_defence_player_state (delegate `ShowEndGameText`)))

(event `InputAxis|ZoomLevel`
  (params (AxisValue :type "Float (single-precision)"))
  ;[1 1 1] Intended to be a zoon controller
)

(event `InputAction|MainAction`
  (params (Key :type "Key Structure"))
  ;[1 1 1] Main mouse action
  (:`Pressed`
    (switch `/Game/Fargor/Characters/Player/PlayerModes` (`self.Mode`)
      (:`NewEnumerator0`
        (`self.Fire Weapon`) ; Deals with attacks
      )
      (:`NewEnumerator1`
        ;[1 1 1] Deals with building
        (`self.BuildTower` (`.Location` (`GameplayStatics.BreakHitResult` (`self.GetHitResultUnderCursorByChannel` "TraceTypeQuery1"))))))))

(event `InputAction|SecondaryAction`
  (params (Key :type "Key Structure"))
  ;[1 1 1] Deals with secondary action
  (:`Released`
    (bind _asbp_base_building (cast `/Game/Fargor/Buildings/BP_BaseBuilding` (`.HitActor` (`GameplayStatics.BreakHitResult` (`self.GetHitResultUnderCursorByChannel` "TraceTypeQuery1")))))
    (cast `/Game/Fargor/Buildings/Core/BP_Core` _asbp_base_building
      (:`CastFailed`
        (`self.DemolitionOnServer` _asbp_base_building)))))

(event `ShowEndGameText`
  (params (DefeatedPlayer :type Name))
  ;[1 1 1] Set up end game screen activation
  (`self.EndTheBloodyGame` DefeatedPlayer))

(event `InputAction|Build_1`
  (params (Key :type "Key Structure"))
  ;[1 1 1] Deals with building
  ;;[1 1 1] Set to building mode and the building
  (:`Pressed`
    (set `self.BuildingToBuild` "NewEnumerator0")
    (bind _asbp_player (cast `/Game/Fargor/Characters/Player/BP_Player` (`self.K2_GetPawn`) :!label _label))
    (if (not (or (`/Game/Fargor/Characters/Player/BP_Player.Dead` _asbp_player) (>= (`self.Towers`) (`self.MaxTowers`))))
      (set `self.Mode` "NewEnumerator1"))))

(event `InputAction|Build_2`
  (params (Key :type "Key Structure"))
  ;[1 1 1] Deals with building
  ;;[1 1 1] Set to building mode and the building
  (:`Pressed`
    (set `self.BuildingToBuild` "NewEnumerator1")
    (goto _label)))

(event `BuildOnServer`
  (params (Target :type "/Game/Fargor/TowerGameMode/BP_TowerDefenceGameState Object Reference") (Building :type "/Game/Fargor/Buildings/Buildings Enum" :default "NewEnumerator3") (Position :type "Transform Structure") (Owner :type "Actor Object Reference"))
  ;[1 1 1] Deals with building
  (switch `/Game/Fargor/Buildings/Buildings` Building
    (:`NewEnumerator0`
      (`/Game/Fargor/TowerGameMode/BP_TowerDefenceGameState.BuildTower` Target Building Position Owner (`self.TargetForAttack`)))
    (:`NewEnumerator1`
      (`/Game/Fargor/TowerGameMode/BP_TowerDefenceGameState.BuildTower` Target Building Position Owner null :!label _label_2))
    (:`NewEnumerator2`
      (goto _label_2)))
  (`/Engine/EditorBlueprintResources/StandardMacros.IncrementInt` (`self.Towers`)))

(event `InputAction|Build_3`
  (params (Key :type "Key Structure"))
  ;[1 1 1] Deals with building
  ;;[1 1 1] Set to building mode and the building
  (:`Pressed`
    (set `self.BuildingToBuild` "NewEnumerator2")
    (goto _label)))

(event `EndTheBloodyGame`
  (params (DefeatedPlayer :type Name))
  ;[1 1 1] The process of showing the end screen starts on the death of a core(in the dead core) passes through  the game state that calls an player state event dispatcher that activates this event on the player controller (I'm sorry for this mess)
  (`/Game/Fargor/UI/Game/HUD/TowerDefenceUI.BringUpEndGameText` (`self.Viewport`) DefeatedPlayer))

(event `DemolitionOnServer`
  (params (Target :type "/Game/Fargor/Buildings/BP_BaseBuilding Object Reference"))
  ;[1 1 1] Demolish a tower
  (if (and (== (`|GetArrayItem` (`Actor.Tags` Target)) (`|GetArrayItem` (`self.Tags`))) (> (`self.Towers`) 0))
    (`/Engine/EditorBlueprintResources/StandardMacros.DecrementInt` (`self.Towers`)
      (:`  `
        (`/Game/Fargor/Buildings/BP_BaseBuilding.Death` Target)))))

(fn `BuildTower`
  (params (Location :type "Vector Structure"))
  (bind _asbp_tower_defence_game_state (cast `/Game/Fargor/TowerGameMode/BP_TowerDefenceGameState` (`GameplayStatics.GetGameState`)))
  (`self.BuildOnServer` _asbp_tower_defence_game_state (`self.BuildingToBuild`) (`KismetMathLibrary.MakeTransform` Location (`KismetMathLibrary.MakeRotator` 0.0 0.0 (`KismetMathLibrary.RandomFloatInRange` 0.0 360.0))) self)
  (set `self.Mode` "NewEnumerator0"))

(fn `CalculatePlayerTurn`
  (bind _returnvalue (`self.K2_GetPawn`))
  (if (`KismetSystemLibrary.IsValid` _returnvalue)
    (bind _asbp_player (cast `/Game/Fargor/Characters/Player/BP_Player` _returnvalue))
    (`/Game/Fargor/Characters/Player/BP_Player.PlayerTurn_Event` _asbp_player (`KismetMathLibrary.RInterpTo` (`SceneComponent.K2_GetComponentRotation` (`/Game/Fargor/Characters/BP_BaseCharacter.Cube` _asbp_player)) (`KismetMathLibrary.MakeRotator` 0.0 0.0 (.yaw (`KismetMathLibrary.FindLookAtRotation` (`self.K2_GetActorLocation` (`self.K2_GetPawn`)) (`.Location` (`GameplayStatics.BreakHitResult` (`self.GetHitResultUnderCursorByChannel` "TraceTypeQuery1")))))) 0.05 4.0))))

(fn `Fire Weapon`
  (bind _asbp_player (cast `/Game/Fargor/Characters/Player/BP_Player` (`self.K2_GetPawn`)))
  (if (not (`/Game/Fargor/Characters/Player/BP_Player.Dead` _asbp_player))
    (bind _bp_baseattack (`/Game/Fargor/Characters/BP_BaseCharacter.BP_BaseAttack` _asbp_player))
    (set `/Game/Fargor/Components/Attacks/BP_BaseAttack.Damage` (`/Game/Fargor/Characters/BP_BaseCharacter.BaseDamage` _asbp_player) _bp_baseattack)
    (set `/Game/Fargor/Components/Attacks/BP_BaseAttack.BulletLifetime` (`/Game/Fargor/Characters/BP_BaseCharacter.BulletLifetime` _asbp_player) _bp_baseattack)
    (`/Game/Fargor/Components/Attacks/BP_BaseAttack.AttackOnServer` _bp_baseattack)))

(fn `UserConstructionScript`)